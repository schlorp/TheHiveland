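; AK47 weapon Blueprint: a full-auto rifle that attaches to the player's first-person mesh on overlap if no weapon is equipped.
; Pickup binds the player's use, reload and stop-fire events to the gun.
; A looping timer drives camera line-trace shots that spend magazine ammo, apply point damage and spawn effects plus randomly rotated bullet-hole decals.
; Reloading uses a DoOnce-guarded montage and delay to refill the magazine from reserve ammo, with an infinite-ammo option.
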(event OnComponentBeginOverlap(SphereCollision)
  (params (OverlappedComponent :type Primitive%20Component%20Object%20Reference) (OtherActor :type Actor%20Object%20Reference) (OtherComp :type Primitive%20Component%20Object%20Reference) (OtherBodyIndex :type Integer) (bFromSweep :type Boolean) (SweepResult :type Hit%20Result%20Structure%20%28by%20ref%29))
  ;[1 1 1] Cast to Player
  (bind _asbp_player (Utilities|Casting|CastToBP_Player OtherActor))
  (Variables|Default|SetAs%20BP%20Player _asbp_player)
  (if (Variables|/Game/Player/Blueprints/BP_Player.BP_Player_C|GetWeaponEquiped? (Variables|Default|GetAs%20BP%20Player)) ; Checks if player has a weapon equiped
    (Development|PrintString "already equied weapon")
    (else
      ;[1 1 1] Attaches component to player
      (Transformation|AttachComponentToComponent self (Variables|/Game/Player/Blueprints/BP_Player.BP_Player_C|GetFirstPersonMesh (Variables|Default|GetAs%20BP%20Player)) "AR_Socket" "SnapToTarget" "SnapToTarget" "SnapToTarget" true)
      (Variables|/Game/Player/Blueprints/BP_Player.BP_Player_C|SetWeaponEquiped? (Variables|Default|GetAs%20BP%20Player) true)
      ;[1 0.06871 0.9013] Bind Events
      ;;[1 1 1] Bind Use Fire
      (EventDispatchers|BindEventtoOnUseItem (Variables|Default|GetAs%20BP%20Player) (EventDispatchers|CreateEvent :!event FireGun))
      ;;[1 1 1] Bind Reload
      (EventDispatchers|BindEventtoOnReload (Variables|Default|GetAs%20BP%20Player) (EventDispatchers|CreateEvent :!event Reload))
      ;;[1 1 1] Bind Stop fire
      (EventDispatchers|BindEventtoStopFire (Variables|Default|GetAs%20BP%20Player) (delegate EventStopFiring)))))

(event EventFireGun
  (bind _as_bp_player (Variables|Default|GetAs%20BP%20Player))
  ;[1 0 0] Fire Gun Event
  ;;[1 1 1] Full Auto of Gun
  (if (== (Variables|Ammo|GetCurrent%20Mag) 0)
    (Utilities|Time|ClearandInvalidateTimerbyHandle (Variables|Default|GetGun%20Timer))
    (Audio|PlaySoundatLocation "/Game/Weapons/AK47/Sounds/DryFireCue.DryFireCue" "0, 0, 0" "0, 0, 0" 1.0 1.0 0.0 0 0 0 0)
    (else
      (bind _returnvalue (Utilities|Time|SetTimerbyEvent (delegate EventFireGun) (Variables|Firing|GetFire%20Rate) true))
      (Variables|Default|SetGun%20Timer _returnvalue)
      ;;[1 1 1] Fire Logic
      (Animation|Montage|PlayMontage (Variables|Default|GetAK) "/Game/Weapons/AK47/Anim/AK_FIRE2_Montage.AK_FIRE2_Montage"
        (:then
          (bind (_camrotation _camlocation _camendlocation) (Default|GetCamRot+Loc _as_bp_player))
          (bind (_outhit _returnvalue_2) (Collision|LineTraceByChannel _camlocation _camendlocation "TraceTypeQuery2" true (Utilities|Array|MakeArray _as_bp_player) "None"))
          (CallFunction|UseAmmo self)
          (Audio|PlaySoundatLocation "/Game/Weapons/AK47/Sounds/GunShotCue.GunShotCue" "0, 0, 0" "0, 0, 0" 1.0 1.0 0.0 0 0 0 0)
          (Effects|SpawnEmitterAttached "/Game/Weapons/MuzzleFlash/Effects/P_BackPack_MuzzleFlash.P_BackPack_MuzzleFlash" (Variables|Default|GetMuzzleFlash) "None" "0, 0, 0" "0, 0, 0" "0.100000,0.100000,0.100000")
          ;;[1 1 1] Dmg Locig
          (if _returnvalue_2
            (Game|Damage|ApplyPointDamage (.HitActor (Collision|BreakHitResult _outhit)) 3e+01 (Variables|/Game/Player/Blueprints/BP_Player.BP_Player_C|GetCameraLocation (Variables|Default|GetAs%20BP%20Player)) _outhit (Game|GetInstigatorController) self "/Script/Engine.DamageType")
            (Effects|SpawnEmitteratLocation "/Game/Weapons/BulletRelated/WallImpact/FX/P_Impact_Stone_Medium_01.P_Impact_Stone_Medium_01" (.Location (Collision|BreakHitResult _outhit)))
            ;;[1 1 1] BulletHole Spawing
            (bind _returnvalue_3 (CallFunction|RandomRotCalc (.ImpactNormal (Collision|BreakHitResult _outhit))))
            (bind _returnvalue_4 (Rendering|Decal|SpawnDecalatLocation "/Game/Weapons/BulletRelated/BulletHole/BulletHole_Mat.BulletHole_Mat" "5.000000,5.000000,5.000000" (.ImpactPoint (Collision|BreakHitResult _outhit)) _returnvalue_3 1e+01))
            (bind _output_get (Variables|Default|SetSpawned%20Decal _returnvalue_4))
            (Transformation|SetWorldLocationAndRotation _output_get (.ImpactPoint (Collision|BreakHitResult _outhit)) _returnvalue_3 false false)))))))

(event EventStopFiring
  ;[1 0.06871 0.9013] Bind Events
  ;;[1 1 1] Bind Stop fire
  (Utilities|Time|ClearandInvalidateTimerbyHandle (Variables|Default|GetGun%20Timer))
  (Audio|Components|Audio|Stop (Variables|Default|GetAK)))

(event EventReload
  ;[1 1 1] Reloading
  (if (and (!= 30 (Variables|Ammo|GetCurrent%20Mag)) (!= (Variables|Ammo|GetAmmo) 0))
    (Utilities|FlowControl|DoOnce false :!label _label
      (:Completed
        (Variables|/Game/Player/Blueprints/BP_Player.BP_Player_C|SetReloading? (Variables|Default|GetAs%20BP%20Player) true)
        (Audio|PlaySound2D "/Game/Weapons/AK47/Sounds/ReloadSound.ReloadSound" 1.0 1.0 0.0 0 0)
        (Animation|Montage|PlayMontage (Variables|/Game/Player/Blueprints/BP_Player.BP_Player_C|GetFirstPersonMesh (Variables|Default|GetAs%20BP%20Player)) "/Game/Player/Animations/Montages/FP_Reload_Montage.FP_Reload_Montage"
          (:then
            _)
          (:OnCompleted
            _))
        (Utilities|FlowControl|Delay 2.1)
        (CallFunction|ReloadRifle)
        (Variables|/Game/Player/Blueprints/BP_Player.BP_Player_C|SetReloading? (Variables|Default|GetAs%20BP%20Player) false)
        (goto _label Reset)))))

(fn ConstructionScript
  (|CallParentFunction))

(fn RandomRotCalc
  (params (In%20Vec :type Vector))
  (bind _returnvalue (Math|Conversions|RotationFromXVector In%20Vec))
  (bind _returnvalue_2 (Math|Random|RandomFloatinRange 0.0 3.6e+02))
  (bind (_x _y _z) (Math|Rotator|BreakRotIntoAxes _returnvalue))
  (return (Math|Rotator|MakeRotationfromAxes _x (Math|Vector|RotateVectorAroundAxis _y _returnvalue_2 _x) (Math|Vector|RotateVectorAroundAxis _z _returnvalue_2 _x))))

(fn UseAmmo
  (Variables|Ammo|SetCurrent%20Mag (Math|Integer|Clamp(Integer) (- (Variables|Ammo|GetCurrent%20Mag) 1) 0 30)))

(fn ReloadRifle
  (LocalVariables|SetTemp%20Ammo (Variables|Ammo|GetAmmo))
  (Variables|Ammo|SetAmmo (Math|Integer|Clamp(Integer) (- (Variables|Ammo|GetAmmo) (- 30 (Variables|Ammo|GetCurrent%20Mag))) 0 (Variables|Ammo|GetAmmo))) ; End Ammo
  (Variables|Ammo|SetCurrent%20Mag (+ (- (LocalVariables|GetTemp%20Ammo) (Variables|Ammo|GetAmmo)) (Variables|Ammo|GetCurrent%20Mag)))
  (if (Variables|Ammo|GetInfiniteAmmo?)
    (Variables|Ammo|SetAmmo 999)))