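; AK47 weapon Blueprint that attaches to the player's first-person mesh on sphere overlap and binds to the player's use, reload and stop-fire events.
; FireGun repeats on a timer for full auto, using ammo and line-tracing from the camera to apply point damage with muzzle, sound and impact effects.
; Bullet-hole decals get randomized rotation around the hit normal.
; Reload is DoOnce-gated, playing a montage before refilling after a fixed delay.
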(event OnComponentBeginOverlap(SphereCollision)
  (params (OverlappedComponent :type Primitive%20Component%20Object%20Reference) (OtherActor :type Actor%20Object%20Reference) (OtherComp :type Primitive%20Component%20Object%20Reference) (OtherBodyIndex :type Integer) (bFromSweep :type Boolean) (SweepResult :type Hit%20Result%20Structure%20%28by%20ref%29))
  (bind _asbp_player (Utilities|Casting|CastToBP_Player OtherActor))
  (bind _output_get (Variables|Default|SetAs%20BP%20Player _asbp_player))
  (Transformation|AttachComponentToComponent self (Variables|/Game/Player/Blueprints/BP_Player.BP_Player_C|GetFirstPersonMesh _output_get) "AR_Socket" "SnapToTarget" "SnapToTarget" "SnapToTarget" true)
  (Variables|/Game/Player/Blueprints/BP_Player.BP_Player_C|SetWeaponEquiped? (Variables|Default|GetAs%20BP%20Player) true)
  ;[1 1 1] Bind Events
  (EventDispatchers|BindEventtoOnUseItem (Variables|Default|GetAs%20BP%20Player) (EventDispatchers|CreateEvent :!event Custom|FireGun))
  (EventDispatchers|BindEventtoOnReload (Variables|Default|GetAs%20BP%20Player) (EventDispatchers|CreateEvent :!event Custom|Reload))
  (EventDispatchers|BindEventtoStopFire (Variables|Default|GetAs%20BP%20Player) (delegate Custom|Stop%20Firing)))

(event Custom|FireGun
  (bind _as_bp_player (Variables|Default|GetAs%20BP%20Player))
  ;[1 1 1] Full Auto of Gun
  (if (== (Variables|/Game/Player/Blueprints/BP_Player.BP_Player_C|GetCurrentMag (Variables|Default|GetAs%20BP%20Player)) 0)
    (Utilities|Time|ClearandInvalidateTimerbyHandle (Variables|Default|GetGun%20TimerRef))
    (Audio|PlaySoundatLocation "/Game/Weapons/AK47/Sounds/DryFireCue.DryFireCue" "0, 0, 0" "0, 0, 0" 1.0 1.0 0.0 0 0 0 0)
    (else
      (bind _returnvalue (Utilities|Time|SetTimerbyEvent (delegate Custom|FireGun) (Variables|Default|GetFireRate) true))
      (Variables|Default|SetGun%20TimerRef _returnvalue)
      ;[1 1 1] Fire Logic
      (Animation|Montage|PlayMontage (Variables|Default|GetAK) "/Game/Weapons/AK47/Anim/AK_FIRE2_Montage.AK_FIRE2_Montage"
        (:then
          (bind (_camrotation _camlocation _camendlocation) (Default|GetCamRot+Loc _as_bp_player))
          (bind (_outhit _returnvalue_2) (Collision|LineTraceByChannel _camlocation _camendlocation "TraceTypeQuery2" true (Utilities|Array|MakeArray _as_bp_player) "None"))
          (Default|UseAmmo (Variables|Default|GetAs%20BP%20Player))
          (Audio|PlaySoundatLocation "/Game/Weapons/AK47/Sounds/GunShotCue.GunShotCue" "0, 0, 0" "0, 0, 0" 1.0 1.0 0.0 0 0 0 0)
          (Effects|SpawnEmitterAttached "/Game/Weapons/MuzzleFlash/Effects/P_BackPack_MuzzleFlash.P_BackPack_MuzzleFlash" (Variables|Default|GetMuzzleFlash) "None" "0, 0, 0" "0, 0, 0" "0.010000,0.010000,0.010000")
          ;[1 1 1] Dmg Locig
          (if _returnvalue_2
            (Game|Damage|ApplyPointDamage (.HitActor (Collision|BreakHitResult _outhit)) 3e+01 (Variables|/Game/Player/Blueprints/BP_Player.BP_Player_C|GetCameraLocation (Variables|Default|GetAs%20BP%20Player)) _outhit (Game|GetInstigatorController) self "/Script/Engine.DamageType")
            (Effects|SpawnEmitteratLocation "/Game/Weapons/BulletRelated/WallImpact/FX/P_Impact_Stone_Medium_01.P_Impact_Stone_Medium_01" (.Location (Collision|BreakHitResult _outhit)))
            ;[1 1 1] BulletHole Spawing
            (bind _returnvalue_3 (CallFunction|RandomRotCalc (.ImpactNormal (Collision|BreakHitResult _outhit))))
            (bind _returnvalue_4 (Rendering|Decal|SpawnDecalatLocation "/Game/Weapons/BulletRelated/BulletHole/BulletHole_Mat.BulletHole_Mat" "5.000000,5.000000,5.000000" (.ImpactPoint (Collision|BreakHitResult _outhit)) _returnvalue_3 1e+01))
            (bind _output_get (Variables|Default|SetSpawnedDecal _returnvalue_4))
            (Transformation|SetWorldLocationAndRotation _output_get (.ImpactPoint (Collision|BreakHitResult _outhit)) _returnvalue_3 false false)))))))

(event Custom|Reload
  (bind _as_bp_player (Variables|Default|GetAs%20BP%20Player))
  (if (and (!= 30 (Variables|/Game/Player/Blueprints/BP_Player.BP_Player_C|GetCurrentMag _as_bp_player)) (!= (Variables|/Game/Player/Blueprints/BP_Player.BP_Player_C|GetAmmo _as_bp_player) 0))
    (Utilities|FlowControl|DoOnce false :!label _label
      (:Completed
        (Variables|/Game/Player/Blueprints/BP_Player.BP_Player_C|SetReloading? (Variables|Default|GetAs%20BP%20Player) true)
        (Audio|PlaySound2D "/Game/Weapons/AK47/Sounds/ReloadSound.ReloadSound" 1.0 1.0 0.0 0 0)
        (Animation|Montage|PlayMontage (Variables|/Game/Player/Blueprints/BP_Player.BP_Player_C|GetFirstPersonMesh (Variables|Default|GetAs%20BP%20Player)) "/Game/Player/Animations/Montages/FP_Reload_Montage.FP_Reload_Montage"
          (:then
            _)
          (:OnCompleted
            _))
        (Utilities|FlowControl|Delay 2.1)
        (Default|Reload (Variables|Default|GetAs%20BP%20Player))
        (Variables|/Game/Player/Blueprints/BP_Player.BP_Player_C|SetReloading? (Variables|Default|GetAs%20BP%20Player) false)
        (goto _label Reset)))))

(event Custom|Stop%20Firing
  ;[1 1 1] Bind Events
  (Utilities|Time|ClearandInvalidateTimerbyHandle (Variables|Default|GetGun%20TimerRef))
  (Audio|Components|Audio|Stop (Variables|Default|GetAK)))

(fn ConstructionScript)

(fn RandomRotCalc
  (params (InVec :type Vector))
  (bind _returnvalue (Math|Conversions|RotationFromXVector InVec))
  (bind _returnvalue_2 (Math|Random|RandomFloatinRange 0.0 3.6e+02))
  (bind (_x _y _z) (Math|Rotator|BreakRotIntoAxes _returnvalue))
  (return (Math|Rotator|MakeRotationfromAxes _x (Math|Vector|RotateVectorAroundAxis _y _returnvalue_2 _x) (Math|Vector|RotateVectorAroundAxis _z _returnvalue_2 _x))))