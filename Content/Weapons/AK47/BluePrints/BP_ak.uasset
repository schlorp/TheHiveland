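; AK-47 pickup that attaches to an unarmed player's first-person mesh on overlap and binds to their fire, stop and reload events.
; Full-auto fire re-arms a timer, line-tracing from the camera to apply point damage with muzzle flash, impact effects and randomly rotated bullet-hole decals.
; A DoOnce-gated, delayed reload refills the magazine from reserve ammo, which an infinite-ammo flag replenishes.
; Magazine, reserve and fire rate are set in the construction script.
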(event Collision|EventActorBeginOverlap
  (params (OtherActor :type Actor%20Object%20Reference))
  ;[1 1 1] Cast to Player
  (bind _asbp_player (Utilities|Casting|CastToBP_Player OtherActor))
  (Variables|Default|SetAs%20BP%20Player_1 _asbp_player)
  (if (Variables|/Game/Player/Blueprints/BP_Player.BP_Player_C|GetWeaponEquiped? (Variables|Default|GetAs%20BP%20Player_1)) ; Checks if player has a weapon equiped
    (Development|PrintString "already equied weapon")
    (else
      ;[1 1 1] Attaches component to player
      (Transformation|AttachComponentToComponent self (Variables|/Game/Player/Blueprints/BP_Player.BP_Player_C|GetFirstPersonMesh (Variables|Default|GetAs%20BP%20Player_1)) "AR_Socket" "SnapToTarget" "SnapToTarget" "SnapToTarget" true)
      (Variables|/Game/Player/Blueprints/BP_Player.BP_Player_C|SetWeaponEquiped? (Variables|Default|GetAs%20BP%20Player_1) true)
      ;[1 0.06871 0.9013] Bind Events
      ;;[1 1 1] Bind Use Fire
      (EventDispatchers|BindEventtoOnUseItem (Variables|Default|GetAs%20BP%20Player_1) (EventDispatchers|CreateEvent :!event FireGun))
      ;;[1 1 1] Bind Reload
      (EventDispatchers|BindEventtoOnReload (Variables|Default|GetAs%20BP%20Player_1) (EventDispatchers|CreateEvent :!event Reload))
      ;;[1 1 1] Bind Stop fire
      (EventDispatchers|BindEventtoStopFire (Variables|Default|GetAs%20BP%20Player_1) (delegate EventStopFiring))
      (Variables|/Game/Player/Blueprints/BP_Player.BP_Player_C|SetAK%20Equiped? (Variables|Default|GetAs%20BP%20Player_1) true))))

(event EventFireGun
  (bind _as_bp_player_1 (Variables|Default|GetAs%20BP%20Player_1))
  ;[1 0 0] Fire Gun Event
  ;;[1 1 1] Full Auto of Gun
  (if (== (Variables|Default|GetCurrent%20Mag) 0)
    (Utilities|Time|ClearandInvalidateTimerbyHandle (Variables|Firing|GetGun%20Timer))
    (Audio|PlaySound2D "/Game/Weapons/AK47/Sounds/DryFireCue.DryFireCue" 1.0 1.0 0.0 0 0)
    (else
      (bind _returnvalue (Utilities|Time|SetTimerbyEvent (delegate EventFireGun) (Variables|Default|GetFire%20Rate) true))
      (Variables|Firing|SetGun%20Timer _returnvalue)
      ;;[1 1 1] Fire Logic
      (Animation|Montage|PlayMontage (Variables|Default|GetAK) "/Game/Weapons/AK47/Anim/AK_FIRE2_Montage.AK_FIRE2_Montage"
        (:then
          (bind (_camrotation _camlocation _camendlocation) (Default|GetCamRot+Loc _as_bp_player_1))
          (bind (_outhit _returnvalue_2) (Collision|LineTraceByChannel _camlocation _camendlocation "TraceTypeQuery2" true (Utilities|Array|MakeArray _as_bp_player_1) "None"))
          (CallFunction|UseAmmo self)
          (Audio|PlaySoundatLocation "/Game/Weapons/AK47/Sounds/GunShotCue.GunShotCue" "0, 0, 0" "0, 0, 0" 1.0 1.0 0.0 0 0 0 0)
          (Effects|SpawnEmitterAttached "/Game/Weapons/MuzzleFlash/Effects/P_BackPack_MuzzleFlash.P_BackPack_MuzzleFlash" (Variables|Default|GetMuzzleFlash) "None" "0, 0, 0" "0, 0, 0" "0.100000,0.100000,0.100000")
          ;;[1 1 1] Dmg Locig
          (if _returnvalue_2
            (Game|Damage|ApplyPointDamage (.HitActor (Collision|BreakHitResult _outhit)) 3e+01 (Variables|/Game/Player/Blueprints/BP_Player.BP_Player_C|GetCameraLocation (Variables|Default|GetAs%20BP%20Player_1)) _outhit (Game|GetInstigatorController) self "/Script/Engine.DamageType")
            (Effects|SpawnEmitteratLocation "/Game/Weapons/BulletRelated/WallImpact/FX/P_Impact_Stone_Medium_01.P_Impact_Stone_Medium_01" (.Location (Collision|BreakHitResult _outhit)))
            ;;[1 1 1] BulletHole Spawing
            (bind _random_rotation (CallFunction|RandomRotCalc (.ImpactNormal (Collision|BreakHitResult _outhit))))
            (bind _returnvalue_3 (Rendering|Decal|SpawnDecalatLocation "/Game/Weapons/BulletRelated/BulletHole/BulletHole_Mat.BulletHole_Mat" "5.000000,5.000000,5.000000" (.ImpactPoint (Collision|BreakHitResult _outhit)) _random_rotation 1e+01))
            (bind _output_get (Variables|Default|SetSpawned%20Decal _returnvalue_3))
            (Transformation|SetWorldLocationAndRotation _output_get (.ImpactPoint (Collision|BreakHitResult _outhit)) _random_rotation false false)))))))

(event EventStopFiring
  ;[1 0.06871 0.9013] Bind Events
  ;;[1 1 1] Bind Stop fire
  (Utilities|Time|ClearandInvalidateTimerbyHandle (Variables|Firing|GetGun%20Timer))
  (Audio|Components|Audio|Stop (Variables|Default|GetAK)))

(event EventReload
  ;[1 1 1] Reloading
  (if (and (!= 30 (Variables|Default|GetCurrent%20Mag)) (!= (Variables|Default|GetAmmo) 0))
    (Utilities|FlowControl|DoOnce false :!label _label
      (:Completed
        (Variables|/Game/Player/Blueprints/BP_Player.BP_Player_C|SetReloading? (Variables|Default|GetAs%20BP%20Player_1) true)
        (Audio|PlaySound2D "/Game/Weapons/AK47/Sounds/ReloadSound.ReloadSound" 1.0 1.0 0.0 0 0)
        (Animation|Montage|PlayMontage (Variables|/Game/Player/Blueprints/BP_Player.BP_Player_C|GetFirstPersonMesh (Variables|Default|GetAs%20BP%20Player_1)) "/Game/Player/Animations/Montages/FP_Reload_Montage.FP_Reload_Montage"
          (:then
            _)
          (:OnCompleted
            _))
        (Utilities|FlowControl|Delay 2.1)
        (CallFunction|ReloadRifle)
        (Variables|/Game/Player/Blueprints/BP_Player.BP_Player_C|SetReloading? (Variables|Default|GetAs%20BP%20Player_1) false)
        (goto _label Reset)))))

(fn ConstructionScript
  (|CallParentFunction)
  (Variables|Default|SetCurrent%20Mag 30)
  (Variables|Default|SetAmmo 60)
  (Variables|Default|SetFire%20Rate 0.08)
  (Development|PrintString "Setting  varibakes"))

(fn RandomRotCalc
  (params (In%20Vec :type Vector))
  (bind _returnvalue (Math|Conversions|RotationFromXVector In%20Vec))
  (bind _returnvalue_2 (Math|Random|RandomFloatinRange 0.0 3.6e+02))
  (bind (_x _y _z) (Math|Rotator|BreakRotIntoAxes _returnvalue))
  (return (Math|Rotator|MakeRotationfromAxes _x (Math|Vector|RotateVectorAroundAxis _y _returnvalue_2 _x) (Math|Vector|RotateVectorAroundAxis _z _returnvalue_2 _x))))

(fn UseAmmo
  (Variables|Default|SetCurrent%20Mag (Math|Integer|Clamp(Integer) (- (Variables|Default|GetCurrent%20Mag) 1) 0 30)))

(fn ReloadRifle
  (LocalVariables|SetTemp%20Ammo (Variables|Default|GetAmmo)) ; Start Ammo
  (Variables|Default|SetAmmo (Math|Integer|Clamp(Integer) (- (Variables|Default|GetAmmo) (- 30 (Variables|Default|GetCurrent%20Mag))) 0 (Variables|Default|GetAmmo))) ; End Ammo
  (Variables|Default|SetCurrent%20Mag (+ (- (LocalVariables|GetTemp%20Ammo) (Variables|Default|GetAmmo)) (Variables|Default|GetCurrent%20Mag)))
  (if (Variables|Ammo|GetInfiniteAmmo?)
    (Variables|Default|SetAmmo 990)))