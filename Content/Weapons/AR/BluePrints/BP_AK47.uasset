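; BP_AK47 is an AK-47 pickup that attaches to the first-person mesh of an overlapping BP_Player and binds to that player's item-use, reload and stop-fire events.
; A looping timer drives automatic fire until stopped or the magazine empties.
; Each shot uses player ammo, plays effects and applies point damage through a camera line trace.
; Reload plays a montage behind a DoOnce, then refills through the player after a delay.
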(event OnComponentBeginOverlap(SphereCollision)
  (params (OverlappedComponent :type Primitive%20Component%20Object%20Reference) (OtherActor :type Actor%20Object%20Reference) (OtherComp :type Primitive%20Component%20Object%20Reference) (OtherBodyIndex :type Integer) (bFromSweep :type Boolean) (SweepResult :type Hit%20Result%20Structure%20%28by%20ref%29))
  (bind _asbp_player (Utilities|Casting|CastToBP_Player OtherActor))
  (bind _output_get (Variables|Default|SetAs%20BP%20Player _asbp_player))
  (Transformation|AttachComponentToComponent self (Variables|/Game/Player/Blueprints/BP_Player.BP_Player_C|GetFirstPersonMesh _output_get) "AR_Socket" "SnapToTarget" "SnapToTarget" "SnapToTarget" true)
  (EventDispatchers|BindEventtoOnUseItem (Variables|Default|GetAs%20BP%20Player) (EventDispatchers|CreateEvent :!event Custom|FireGun))
  (EventDispatchers|BindEventtoOnReload (Variables|Default|GetAs%20BP%20Player) (EventDispatchers|CreateEvent :!event Custom|Reload))
  (EventDispatchers|BindEventtoStopFire (Variables|Default|GetAs%20BP%20Player) (delegate Custom|Stop%20Firing)))

(event Custom|FireGun
  (if (== (Variables|/Game/Player/Blueprints/BP_Player.BP_Player_C|GetCurrentMag (Variables|Default|GetAs%20BP%20Player)) 0)
    (Utilities|Time|ClearandInvalidateTimerbyHandle (Variables|Default|GetGun%20TimerRef))
    (else
      (bind _returnvalue (Utilities|Time|SetTimerbyEvent (delegate Custom|FireGun) (Variables|Default|GetFireRate) true))
      (Variables|Default|SetGun%20TimerRef _returnvalue)
      ;[1 1 1] Fire Logic
      (Components|Animation|PlayAnimation (Variables|Default|GetAK) "/Game/Weapons/AR/Anim/AK_FIRE2.AK_FIRE2" false)
      (bind (_camrotation _camlocation _camendlocation) (Default|GetCamRot+Loc (Variables|Default|GetAs%20BP%20Player)))
      (bind (_outhit _returnvalue_2) (Collision|LineTraceByChannel _camlocation _camendlocation "TraceTypeQuery2" true (Utilities|Array|MakeArray (Variables|Default|GetAs%20BP%20Player)) "ForDuration"))
      (Default|UseAmmo (Variables|Default|GetAs%20BP%20Player))
      (Audio|PlaySoundatLocation "/Game/Weapons/AR/Sounds/GunShotCue.GunShotCue" "0, 0, 0" "0, 0, 0" 1.0 1.0 0.0 0 0 0 0)
      (Effects|SpawnEmitterAttached "/Game/Weapons/MuzzleFlash/Effects/FX_Monsters/FX_Monster_Gruntling/Master/P_BackPack_MuzzleFlash.P_BackPack_MuzzleFlash" (Variables|/Game/Player/Blueprints/BP_Player.BP_Player_C|GetMuzzleFlash (Variables|Default|GetAs%20BP%20Player)) "None" "0, 0, 0" "0, 0, 0" "0.010000,0.010000,0.010000")
      ;[1 1 1] Dmg Locig
      (if _returnvalue_2
        (Game|Damage|ApplyPointDamage (.HitActor (Collision|BreakHitResult _outhit)) 5.0 (Variables|/Game/Player/Blueprints/BP_Player.BP_Player_C|GetCameraLocation (Variables|Default|GetAs%20BP%20Player)) _outhit (Game|GetInstigatorController) self "/Script/Engine.DamageType")
        (Effects|SpawnEmitteratLocation "/Game/Weapons/WallImpact/FX/P_Impact_Stone_Medium_01.P_Impact_Stone_Medium_01" (.Location (Collision|BreakHitResult _outhit)))))))

(event Custom|Reload
  (if (!= (Variables|/Game/Player/Blueprints/BP_Player.BP_Player_C|GetAmmo (Variables|Default|GetAs%20BP%20Player)) 0)
    (Utilities|FlowControl|DoOnce false :!label _label
      (:Completed
        (Variables|Default|SetReloading? true)
        (Audio|PlaySound2D "/Game/Weapons/AR/Sounds/ReloadSound.ReloadSound" 1.0 1.0 0.0 0 0)
        (Animation|Montage|PlayMontage (Variables|/Game/Player/Blueprints/BP_Player.BP_Player_C|GetFirstPersonMesh (Variables|Default|GetAs%20BP%20Player)) "/Game/Player/Animations/Montages/FP_Reload_Montage.FP_Reload_Montage"
          (:then
            _)
          (:OnCompleted
            _))
        (Utilities|FlowControl|Delay 2.1)
        (Default|Reload (Variables|Default|GetAs%20BP%20Player))
        (Variables|Default|SetReloading? false)
        (goto _label Reset)))))

(event Custom|Stop%20Firing
  (Utilities|Time|ClearandInvalidateTimerbyHandle (Variables|Default|GetGun%20TimerRef)))

(fn ConstructionScript)