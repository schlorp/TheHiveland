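; Desert Eagle pistol Blueprint that the player can pick up, fire and reload.
; Pickup drops any equipped weapon in its place, attaches to the first-person mesh's pistol socket and binds the player's fire, stop-fire and reload dispatchers.
; Firing line-traces from the camera, applying point damage, effects and randomly rotated bullet-hole decals.
; Reload is DoOnce-gated and delayed, refilling a seven-round magazine from reserve ammo, though its full-magazine check compares against 30.
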(event EventBeginPlay
  ;[1 1 1] Getting Player Ref
  (Variables|Default|SetAs%20BP%20Player (.AsBP%20Player (Utilities|Casting|CastToBP_Player (Game|GetPlayerCharacter 0)))))

(event EventFireGun
  (bind _as_bp_player (Variables|Default|GetAs%20BP%20Player))
  ;[1 0 0] Fire Gun Event
  ;;[1 1 1] Full Auto of Gun
  (if (== (Variables|Default|GetCurrent%20Mag) 0)
    (Audio|PlaySound2D "/Game/Weapons/AK47/Sounds/DryFireCue.DryFireCue" 1.0 1.0 0.0 0 0)
    (else
      ;;[1 1 1] Fire Logic
      (Animation|Montage|PlayMontage (Variables|Default|GetGunMesh) "/Game/Weapons/AK47/Anim/AK_FIRE2_Montage.AK_FIRE2_Montage"
        (:then
          (bind (_camrotation _camlocation _camendlocation) (Default|GetCamRot+Loc _as_bp_player))
          (bind (_outhit _returnvalue) (Collision|LineTraceByChannel _camlocation _camendlocation "TraceTypeQuery2" true (Utilities|Array|MakeArray _as_bp_player) "None"))
          (CallFunction|UseAmmo self)
          (Audio|PlaySoundatLocation "/Game/Weapons/Deagle/Sounds/DeagleFire.DeagleFire" "0, 0, 0" "0, 0, 0" 1.0 1.0 0.0 0 0 0 0)
          (Effects|SpawnEmitterAttached "/Game/Weapons/MuzzleFlash/Effects/P_BackPack_MuzzleFlash.P_BackPack_MuzzleFlash" (Variables|Default|GetMuzzleFlash) "None" "0, 0, 0" "0, 0, 0" "0.100000,0.100000,0.100000")
          ;;[1 1 1] Dmg Locig
          (if _returnvalue
            (Game|Damage|ApplyPointDamage (.HitActor (Collision|BreakHitResult _outhit)) (Variables|Default|GetDamage) (Variables|/Game/Player/Blueprints/BP_Player.BP_Player_C|GetCameraLocation (Variables|Default|GetAs%20BP%20Player)) _outhit (Game|GetInstigatorController) self "/Script/Engine.DamageType")
            (Effects|SpawnEmitteratLocation "/Game/Weapons/BulletRelated/WallImpact/FX/P_Impact_Stone_Medium_01.P_Impact_Stone_Medium_01" (.Location (Collision|BreakHitResult _outhit)))
            ;;[1 1 1] BulletHole Spawing
            (bind _random_rotation (CallFunction|RandomRotCal (.ImpactNormal (Collision|BreakHitResult _outhit))))
            (bind _returnvalue_2 (Rendering|Decal|SpawnDecalatLocation "/Game/Weapons/BulletRelated/BulletHole/BulletHole_Mat.BulletHole_Mat" "5.000000,5.000000,5.000000" (.ImpactPoint (Collision|BreakHitResult _outhit)) _random_rotation 1e+01))
            (bind _output_get (Variables|Default|SetSpawnedDecal _returnvalue_2))
            (Transformation|SetWorldLocationAndRotation _output_get (.ImpactPoint (Collision|BreakHitResult _outhit)) _random_rotation false false)))))))

(event EventStopFiring
  ;[1 0.06871 0.9013] Bind Events
  ;;[1 1 1] Bind Stop fire
  (Audio|Components|Audio|Stop (Variables|Default|GetGunMesh)))

(event EventReload
  ;[1 1 1] Reloading
  (if (and (!= 30 (Variables|Default|GetCurrent%20Mag)) (!= (Variables|Default|GetAmmo) 0))
    (Utilities|FlowControl|DoOnce false :!label _label
      (:Completed
        (Variables|/Game/Player/Blueprints/BP_Player.BP_Player_C|SetReloading? (Variables|Default|GetAs%20BP%20Player) true)
        (Audio|PlaySound2D "/Game/Weapons/Deagle/Sounds/DeagleReload.DeagleReload" 1.0 1.0 0.0 0 0)
        (Animation|Montage|PlayMontage (Variables|/Game/Player/Blueprints/BP_Player.BP_Player_C|GetFirstPersonMesh (Variables|Default|GetAs%20BP%20Player)) "/Game/Player/Animations/Montages/FP_Reload_Montage.FP_Reload_Montage"
          (:then
            _)
          (:OnCompleted
            _))
        (Utilities|FlowControl|Delay 2.1)
        (CallFunction|ReloadPistol)
        (Variables|/Game/Player/Blueprints/BP_Player.BP_Player_C|SetReloading? (Variables|Default|GetAs%20BP%20Player) false)
        (goto _label Reset)))))

(event EventPickup
  (bind _as_bp_player (Variables|Default|GetAs%20BP%20Player))
  (bind _as_bp_player_2 (Variables|Default|GetAs%20BP%20Player))
  (bind _defaultsceneroot (Variables|Default|GetDefaultSceneRoot))
  ;[1 1 1] Pick Up Event
  (Utilities|IsValid (Variables|/Game/Player/Blueprints/BP_Player.BP_Player_C|GetEquipedWeapon (Variables|Default|GetAs%20BP%20Player))
    (:Is%20Valid
      (Development|PrintString "Hello")
      (Transformation|DetachFromActor (Variables|/Game/Player/Blueprints/BP_Player.BP_Player_C|GetEquipedWeapon (Variables|Default|GetAs%20BP%20Player)) "KeepRelative" "KeepRelative" "KeepRelative")
      (Transformation|SetActorLocationAndRotation (Variables|/Game/Player/Blueprints/BP_Player.BP_Player_C|GetEquipedWeapon (Variables|Default|GetAs%20BP%20Player)) (Transformation|GetWorldLocation _defaultsceneroot) (Transformation|GetWorldRotation _defaultsceneroot))
      (Development|PrintString "Detaching"))
    (:Is%20Not%20Valid
      _))
  (Variables|/Game/Player/Blueprints/BP_Player.BP_Player_C|SetEquipedWeapon _as_bp_player_2 self)
  (Transformation|AttachComponentToComponent (Variables|/Game/Player/Blueprints/BP_Player.BP_Player_C|GetFirstPersonMesh _as_bp_player_2) "Pistol_Socket" "SnapToTarget" "SnapToTarget" "SnapToTarget" true)
  (Variables|/Game/Player/Blueprints/BP_Player.BP_Player_C|SetWeaponEquiped? (Variables|Default|GetAs%20BP%20Player) true)
  ;[1 0.06871 0.9013] Bind Events
  ;;[1 1 1] Bind Use Fire
  (EventDispatchers|BindEventtoOnUseItem _as_bp_player (EventDispatchers|CreateEvent :!event FireGun))
  ;;[1 1 1] Bind Reload
  (EventDispatchers|BindEventtoOnReload _as_bp_player (EventDispatchers|CreateEvent :!event Reload))
  ;;[1 1 1] Bind Stop fire
  (EventDispatchers|BindEventtoStopFire _as_bp_player (delegate EventStopFiring))
  (Variables|/Game/Player/Blueprints/BP_Player.BP_Player_C|SetPistol2%20Equiped? (Variables|Default|GetAs%20BP%20Player) true))

(fn ConstructionScript
  (|CallParentFunction))

(fn ReloadPistol
  (LocalVariables|SetTemp%20Ammo (Variables|Default|GetAmmo))
  (Variables|Default|SetAmmo (Math|Integer|Clamp(Integer) (- (Variables|Default|GetAmmo) (- 7 (Variables|Default|GetCurrent%20Mag))) 0 (Variables|Default|GetAmmo)))
  (Variables|Default|SetCurrent%20Mag (+ (- (LocalVariables|GetTemp%20Ammo) (Variables|Default|GetAmmo)) (Variables|Default|GetCurrent%20Mag)))
  (if (Variables|Ammo|GetInfinite%20Ammo?)
    (Variables|Default|SetAmmo 999)))

(fn UseAmmo
  (Variables|Default|SetCurrent%20Mag (Math|Integer|Clamp(Integer) (- (Variables|Default|GetCurrent%20Mag) 1) 0 30)))

(fn RandomRotCal
  (params (InVec :type Vector))
  (bind _returnvalue (Math|Conversions|RotationFromXVector InVec))
  (bind _returnvalue_2 (Math|Random|RandomFloatinRange 0.0 3.6e+02))
  (bind (_x _y _z) (Math|Rotator|BreakRotIntoAxes _returnvalue))
  (return (Math|Rotator|MakeRotationfromAxes _x (Math|Vector|RotateVectorAroundAxis _y _returnvalue_2 _x) (Math|Vector|RotateVectorAroundAxis _z _returnvalue_2 _x))))