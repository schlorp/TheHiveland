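; M1911 pistol pickup that attaches to BP_Player's first-person mesh on overlap if unarmed, then binds to the player's fire, reload and stop events.
; Firing runs a camera line trace, applies point damage, spends ammo, plays effects and spawns randomly rotated bullet-hole decals.
; Reload is DoOnce-gated and delayed, refilling the seven-round magazine from reserve, with optional infinite ammo.
; Its full-magazine check compares against 30, and FireGun itself never checks remaining ammo.
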(event EventBeginPlay
  ;[1 1 1] Hides The Extra Mag in the model
  (Components|SkinnedMesh|HideBonebyName (Variables|Default|GetM19) "MagExtended_001" "PBO_None"))

(event EventReload
  ;[1 1 1] Reloading
  (if (and (!= 30 (Variables|Default|GetCurrent%20Mag)) (!= (Variables|Default|GetAmmo) 0))
    (Utilities|FlowControl|DoOnce false :!label _label
      (:Completed
        (Variables|/Game/Player/Blueprints/BP_Player.BP_Player_C|SetReloading? (Variables|Default|GetAs%20BP%20Player) true)
        (Audio|PlaySound2D "/Game/Weapons/M1911/Sounds/ColtReload.ColtReload" 1.0 1.0 0.0 0 0)
        (Animation|Montage|PlayMontage (Variables|/Game/Player/Blueprints/BP_Player.BP_Player_C|GetFirstPersonMesh (Variables|Default|GetAs%20BP%20Player)) 0 ; Remember to Create Pistol Montage
          (:then
            _)
          (:OnCompleted
            _))
        (Utilities|FlowControl|Delay 2.0)
        (CallFunction|ReloadPistol)
        (Variables|/Game/Player/Blueprints/BP_Player.BP_Player_C|SetReloading? (Variables|Default|GetAs%20BP%20Player) false)
        (goto _label Reset)))))

(event Collision|EventActorBeginOverlap
  (params (OtherActor :type Actor%20Object%20Reference))
  ;[1 1 1] Cast to Player
  (bind _asbp_player (Utilities|Casting|CastToBP_Player OtherActor))
  (bind _output_get (Variables|Default|SetAs%20BP%20Player _asbp_player))
  (if (Variables|/Game/Player/Blueprints/BP_Player.BP_Player_C|GetWeaponEquiped? _output_get)
    (Development|PrintString "Already Equiped Weapon")
    (else
      ;[1 1 1] Attaches component to player
      (Transformation|AttachComponentToComponent (Variables|/Game/Player/Blueprints/BP_Player.BP_Player_C|GetFirstPersonMesh (Variables|Default|GetAs%20BP%20Player)) "AR_Socket" "SnapToTarget" "SnapToTarget" "SnapToTarget" true)
      (Variables|/Game/Player/Blueprints/BP_Player.BP_Player_C|SetWeaponEquiped? (Variables|Default|GetAs%20BP%20Player) true)
      ;[1 0.06871 0.9013] Bind Events
      ;;[1 1 1] Bind Use Fire
      (EventDispatchers|BindEventtoOnUseItem (Variables|Default|GetAs%20BP%20Player) (EventDispatchers|CreateEvent :!event FireGun))
      ;;[1 1 1] Bind Reload
      (EventDispatchers|BindEventtoOnReload (Variables|Default|GetAs%20BP%20Player) (EventDispatchers|CreateEvent :!event Reload))
      ;;[1 1 1] Bind Stop fire
      (EventDispatchers|BindEventtoStopFire (Variables|Default|GetAs%20BP%20Player) (delegate EventStopFiring))
      (Variables|/Game/Player/Blueprints/BP_Player.BP_Player_C|SetPistol1%20Equiped? (Variables|Default|GetAs%20BP%20Player) true))))

(event EventStopFiring
  ;[1 0.06871 0.9013] Bind Events
  ;;[1 1 1] Bind Stop fire
  (Audio|Components|Audio|Stop (Variables|Default|GetM19)))

(event EventFireGun
  (bind _as_bp_player (Variables|Default|GetAs%20BP%20Player))
  ;[0.4072 0 0] Fire Gun Event
  ;;[1 1 1] FireLogic
  (Animation|Montage|PlayMontage (Variables|Default|GetM19) 0
    (:then
      (bind (_camrotation _camlocation _camendlocation) (Default|GetCamRot+Loc _as_bp_player))
      (bind (_outhit _returnvalue) (Collision|LineTraceByChannel _camlocation _camendlocation "TraceTypeQuery2" true (Utilities|Array|MakeArray _as_bp_player) "None"))
      (CallFunction|UseAmmo)
      (Audio|PlaySoundatLocation "/Game/Weapons/M1911/Sounds/ColtFire.ColtFire" "0, 0, 0" "0, 0, 0" 1.0 1.0 0.0 0 0 0 0)
      (Effects|SpawnEmitterAttached "/Game/Weapons/MuzzleFlash/Effects/P_BackPack_MuzzleFlash.P_BackPack_MuzzleFlash" (Variables|Default|GetMuzzleFlash) "None" "0, 0, 0" "0, 0, 0" "0.100000,0.100000,0.100000")
      ;;[1 1 1] Dmg Logic
      (if _returnvalue
        (Game|Damage|ApplyPointDamage (.HitActor (Collision|BreakHitResult _outhit)) 5.0 (Variables|/Game/Player/Blueprints/BP_Player.BP_Player_C|GetCameraLocation (Variables|Default|GetAs%20BP%20Player)) _outhit (Game|GetInstigatorController) self)
        (Effects|SpawnEmitteratLocation "/Game/Weapons/BulletRelated/WallImpact/FX/P_Impact_Stone_Medium_01.P_Impact_Stone_Medium_01" (.Location (Collision|BreakHitResult _outhit)))
        ;;[1 1 1] Bullet Hole Spawning
        (bind _random_rotation (CallFunction|RandomRotCalc (.ImpactNormal (Collision|BreakHitResult _outhit))))
        (bind _returnvalue_2 (Rendering|Decal|SpawnDecalatLocation "/Game/Weapons/BulletRelated/BulletHole/BulletHole_Mat.BulletHole_Mat" "1.500000,1.500000,1.500000" (.ImpactPoint (Collision|BreakHitResult _outhit)) _random_rotation 1e+01))
        (bind _output_get (Variables|Default|SetSpawned%20Decal _returnvalue_2))
        (Transformation|SetWorldLocationAndRotation _output_get (.ImpactPoint (Collision|BreakHitResult _outhit)) _random_rotation false false)))))

(fn ConstructionScript
  (|CallParentFunction))

(fn RandomRotCalc
  (params (In%20Vec :type Vector))
  (bind _returnvalue (Math|Conversions|RotationFromXVector In%20Vec))
  (bind _returnvalue_2 (Math|Random|RandomFloatinRange 0.0 3.6e+02))
  (bind (_x _y _z) (Math|Rotator|BreakRotIntoAxes _returnvalue))
  (return (Math|Rotator|MakeRotationfromAxes _x (Math|Vector|RotateVectorAroundAxis _y _returnvalue_2 _x) (Math|Vector|RotateVectorAroundAxis _z _returnvalue_2 _x))))

(fn UseAmmo
  (Variables|Default|SetCurrent%20Mag (Math|Integer|Clamp(Integer) (- (Variables|Default|GetCurrent%20Mag) 1) 0 7)))

(fn ReloadPistol
  (LocalVariables|SetTemp%20Ammo (Variables|Default|GetAmmo))
  (Variables|Default|SetAmmo (Math|Integer|Clamp(Integer) (- (Variables|Default|GetAmmo) (- 7 (Variables|Default|GetCurrent%20Mag))) 0 (Variables|Default|GetAmmo)))
  (Variables|Default|SetCurrent%20Mag (+ (- (LocalVariables|GetTemp%20Ammo) (Variables|Default|GetAmmo)) (Variables|Default|GetCurrent%20Mag)))
  (if (Variables|Default|GetInfinite%20Ammo)
    (Variables|Default|SetAmmo 999)))