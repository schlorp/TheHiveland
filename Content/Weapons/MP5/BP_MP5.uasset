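; MP5 submachine gun pickup that attaches to the first-person mesh socket of an overlapping player with no weapon equipped.
; It binds to the player's use, reload and stop-fire events.
; Full-auto fire uses a looping timer and camera line traces, applying point damage, effects and randomly rotated bullet-hole decals.
; Reload plays a montage, then after a delay refills the magazine from reserve ammo, with an infinite-ammo option.
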(event Collision|EventActorBeginOverlap
  (params (OtherActor :type Actor%20Object%20Reference))
  ;[1 1 1] Cast to Player
  (bind _asbp_player (Utilities|Casting|CastToBP_Player OtherActor))
  (Variables|Default|SetAs%20BP%20Player_0 _asbp_player)
  (if (Variables|/Game/Player/Blueprints/BP_Player.BP_Player_C|GetWeaponEquiped? (Variables|Default|GetAs%20BP%20Player_0)) ; Cheks if a weapon is equiped
    (Development|PrintString "already equied weapon")
    (else
      ;[1 1 1] Attaches component to player
      (Transformation|AttachComponentToComponent self (Variables|/Game/Player/Blueprints/BP_Player.BP_Player_C|GetFirstPersonMesh (Variables|Default|GetAs%20BP%20Player_0)) "SMG_Socket" "SnapToTarget" "SnapToTarget" "SnapToTarget" true)
      (Variables|/Game/Player/Blueprints/BP_Player.BP_Player_C|SetWeaponEquiped? (Variables|Default|GetAs%20BP%20Player_0) true)
      ;[1 0 0.8618] Bind Events
      ;;[1 1 1] Bind Use Item
      (EventDispatchers|BindEventtoOnUseItem (Variables|Default|GetAs%20BP%20Player_0) (EventDispatchers|CreateEvent :!event FireGun))
      ;;[1 1 1] Bind Reload
      (EventDispatchers|BindEventtoOnReload (Variables|Default|GetAs%20BP%20Player_0) (EventDispatchers|CreateEvent :!event Reload))
      ;;[1 1 1] Bind Stop Fire
      (EventDispatchers|BindEventtoStopFire (Variables|Default|GetAs%20BP%20Player_0) (delegate EventStopFiring))
      (Variables|/Game/Player/Blueprints/BP_Player.BP_Player_C|SetMP5%20Equiped? (Variables|Default|GetAs%20BP%20Player_0) true))))

(event EventStopFiring
  ;[1 0 0.8618] Bind Events
  ;;[1 1 1] Bind Stop Fire
  (Utilities|Time|ClearandInvalidateTimerbyHandle (Variables|Firing|GetGun%20Timer%20REf))
  (Audio|Components|Audio|Stop (Variables|Default|GetMP5)))

(event EventFireGun
  (bind _as_bp_player_0 (Variables|Default|GetAs%20BP%20Player_0))
  ;[0.776 0 0.0419] Firing
  ;;[1 1 1] Full Auto
  (if (== 0 (Variables|Default|GetCurrent%20Mag))
    (Utilities|Time|ClearandInvalidateTimerbyHandle (Variables|Firing|GetGun%20Timer%20REf))
    (Audio|PlaySound2D "/Game/Weapons/AK47/Sounds/DryFireCue.DryFireCue" 1.0 1.0 0.0 0 0)
    (else
      (bind _returnvalue (Utilities|Time|SetTimerbyEvent (delegate EventFireGun) (Variables|Default|GetFire%20Rate) true))
      (Variables|Firing|SetGun%20Timer%20REf _returnvalue)
      ;;[1 1 1] Fire Logic
      (bind (_camrotation _camlocation _camendlocation) (Default|GetCamRot+Loc _as_bp_player_0))
      (bind (_outhit _returnvalue_2) (Collision|LineTraceByChannel _camlocation _camendlocation "TraceTypeQuery2" true (Utilities|Array|MakeArray _as_bp_player_0) "None"))
      (CallFunction|UseAmmo)
      (Audio|PlaySoundatLocation "/Game/Weapons/MP5/Sound/mp5_fire.mp5_fire" "0, 0, 0" "0, 0, 0" 1.0 1.0 0.0 0 0 0 0)
      (Effects|SpawnEmitterAttached "/Game/Weapons/MuzzleFlash/Effects/P_BackPack_MuzzleFlash.P_BackPack_MuzzleFlash" (Variables|Default|GetMuzzleFlash) "None" "0, 0, 0" "0, 0, 0" "0.100000,0.100000,0.100000")
      ;;[1 1 1] dmg logic
      (if _returnvalue_2
        (Game|Damage|ApplyPointDamage (.HitActor (Collision|BreakHitResult _outhit)) 15.0 (Variables|/Game/Player/Blueprints/BP_Player.BP_Player_C|GetCameraLocation (Variables|Default|GetAs%20BP%20Player_0)) _outhit (Game|GetInstigatorController) self)
        (Effects|SpawnEmitteratLocation "/Game/Weapons/BulletRelated/WallImpact/FX/P_Impact_Stone_Medium_01.P_Impact_Stone_Medium_01" (.Location (Collision|BreakHitResult _outhit)))
        ;;[1 1 1] BulletHole Spawning
        (bind _returnvalue_3 (CallFunction|RandomRotCalc (.ImpactNormal (Collision|BreakHitResult _outhit))))
        (bind _returnvalue_4 (Rendering|Decal|SpawnDecalatLocation "/Game/Weapons/BulletRelated/BulletHole/BulletHole_Mat.BulletHole_Mat" "2.500000,2.500000,2.500000" (.ImpactPoint (Collision|BreakHitResult _outhit)) _returnvalue_3 1e+01))
        (bind _output_get (Variables|Default|SetSpawnedDecal _returnvalue_4))
        (Transformation|SetWorldLocationAndRotation _output_get (.ImpactPoint (Collision|BreakHitResult _outhit)) _returnvalue_3 false false)))))

(event EventReload
  ;[1 1 1] Reload
  (if (and (!= (Variables|Default|GetAmmo) 0) (!= (Variables|Default|GetCurrent%20Mag) 30))
    (Utilities|FlowControl|DoOnce false :!label _label
      (:Completed
        (Variables|/Game/Player/Blueprints/BP_Player.BP_Player_C|SetReloading? (Variables|Default|GetAs%20BP%20Player_0) true)
        (Audio|PlaySound2D "/Game/Weapons/MP5/Sound/ReloadMP5.ReloadMP5" 1.0 1.0 0.0 0 0)
        (Animation|Montage|PlayMontage (Variables|/Game/Player/Blueprints/BP_Player.BP_Player_C|GetFirstPersonMesh (Variables|Default|GetAs%20BP%20Player_0)) "/Game/Player/Animations/Montages/FP_Reload_Montage.FP_Reload_Montage" 0.5
          (:then
            _)
          (:OnCompleted
            _))
        (Utilities|FlowControl|Delay 3.0)
        (CallFunction|ReloadSub)
        (Variables|/Game/Player/Blueprints/BP_Player.BP_Player_C|SetReloading? (Variables|Default|GetAs%20BP%20Player_0) false)
        (goto _label Reset)))))

(fn ConstructionScript
  (|CallParentFunction)
  (Variables|Default|SetCurrent%20Mag 30)
  (Variables|Default|SetAmmo 60)
  (Variables|Default|SetFire%20Rate 0.1))

(fn RandomRotCalc
  (params (InVec :type Vector))
  (bind _returnvalue (Math|Conversions|RotationFromXVector InVec))
  (bind _returnvalue_2 (Math|Random|RandomFloatinRange 0.0 3.6e+02))
  (bind (_x _y _z) (Math|Rotator|BreakRotIntoAxes _returnvalue))
  (return (Math|Rotator|MakeRotationfromAxes _x (Math|Vector|RotateVectorAroundAxis _y _returnvalue_2 _x) (Math|Vector|RotateVectorAroundAxis _z _returnvalue_2 _x))))

(fn UseAmmo
  (Variables|Default|SetCurrent%20Mag (Math|Integer|Clamp(Integer) (- (Variables|Default|GetCurrent%20Mag) 1) 0 30)))

(fn ReloadSub
  (LocalVariables|SetTemp%20Ammo (Variables|Default|GetAmmo))
  (Variables|Default|SetAmmo (Math|Integer|Clamp(Integer) (- (Variables|Default|GetAmmo) (- 30 (Variables|Default|GetCurrent%20Mag))) 0 (Variables|Default|GetAmmo)))
  (Variables|Default|SetCurrent%20Mag (+ (- (LocalVariables|GetTemp%20Ammo) (Variables|Default|GetAmmo)) (Variables|Default|GetCurrent%20Mag)))
  (if (Variables|Ammo|GetInfinite%20Ammo?)
    (Variables|Default|SetAmmo 999)))