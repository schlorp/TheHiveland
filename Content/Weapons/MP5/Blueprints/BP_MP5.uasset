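; MP5 SMG weapon Blueprint that the player picks up for full-auto hitscan fire.
; Pickup swaps out the equipped weapon, attaches to the first-person mesh and binds the player's use, reload and stop-fire dispatchers.
; A looping timer drives firing: camera line traces apply point damage, with muzzle, impact and randomly rotated bullet-hole effects.
; DoOnce-gated reload plays a montage, then refills the magazine from reserve ammo after a delay, optionally infinite.
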(event EventFireGun
  (bind _as_bp_player (Variables|Default|GetAs%20BP%20Player))
  ;[0.776 0 0.0419] Firing
  ;;[1 1 1] Full Auto
  (if (== 0 (Variables|Default|GetCurrent%20Mag))
    (Utilities|Time|ClearandInvalidateTimerbyHandle (Variables|Firing|GetGun%20Timer%20REf))
    (Audio|PlaySound2D "/Game/Weapons/AK47/Sounds/DryFireCue.DryFireCue" 1.0 1.0 0.0 0 0)
    (else
      (bind _returnvalue (Utilities|Time|SetTimerbyEvent (delegate EventFireGun) (Variables|Default|GetFire%20Rate) true))
      (Variables|Firing|SetGun%20Timer%20REf _returnvalue)
      ;;[1 1 1] Fire Logic
      (bind (_camrotation _camlocation _camendlocation) (Default|GetCamRot+Loc _as_bp_player))
      (bind (_outhit _returnvalue_2) (Collision|LineTraceByChannel _camlocation _camendlocation "TraceTypeQuery2" true (Utilities|Array|MakeArray _as_bp_player) "None"))
      (CallFunction|UseAmmo)
      (Audio|PlaySoundatLocation "/Game/Weapons/MP5/Sound/mp5_fire.mp5_fire" "0, 0, 0" "0, 0, 0" 1.0 1.0 0.0 0 0 0 0)
      (Effects|SpawnEmitterAttached "/Game/Weapons/MuzzleFlash/Effects/P_BackPack_MuzzleFlash.P_BackPack_MuzzleFlash" (Variables|Default|GetMuzzleFlash) "None" "0, 0, 0" "0, 0, 0" "0.100000,0.100000,0.100000")
      ;;[1 1 1] dmg logic
      (if _returnvalue_2
        (Game|Damage|ApplyPointDamage (.HitActor (Collision|BreakHitResult _outhit)) (Variables|Default|GetDamage) (Variables|/Game/Player/Blueprints/BP_Player.BP_Player_C|GetCameraLocation (Variables|Default|GetAs%20BP%20Player)) _outhit (Game|GetInstigatorController) self)
        (Effects|SpawnEmitteratLocation "/Game/Weapons/BulletRelated/WallImpact/FX/P_Impact_Stone_Medium_01.P_Impact_Stone_Medium_01" (.Location (Collision|BreakHitResult _outhit)))
        ;;[1 1 1] BulletHole Spawning
        (bind _returnvalue_3 (CallFunction|RandomRotCalc (.ImpactNormal (Collision|BreakHitResult _outhit))))
        (bind _returnvalue_4 (Rendering|Decal|SpawnDecalatLocation "/Game/Weapons/BulletRelated/BulletHole/BulletHole_Mat.BulletHole_Mat" "2.500000,2.500000,2.500000" (.ImpactPoint (Collision|BreakHitResult _outhit)) _returnvalue_3 1e+01))
        (bind _output_get (Variables|Default|SetSpawnedDecal _returnvalue_4))
        (Transformation|SetWorldLocationAndRotation _output_get (.ImpactPoint (Collision|BreakHitResult _outhit)) _returnvalue_3 false false)))))

(event EventBeginPlay
  ;[1 1 1] Getting Player Ref
  (Variables|Default|SetAs%20BP%20Player (.AsBP%20Player (Utilities|Casting|CastToBP_Player (Game|GetPlayerCharacter 0)))))

(event EventStopFiring
  ;[1 0 0.8618] Bind Events
  ;;[1 1 1] Bind Stop Fire
  (Utilities|Time|ClearandInvalidateTimerbyHandle (Variables|Firing|GetGun%20Timer%20REf))
  (Audio|Components|Audio|Stop (Variables|Default|GetMP5)))

(event EventPickup
  (bind _as_bp_player (Variables|Default|GetAs%20BP%20Player))
  (bind _as_bp_player_2 (Variables|Default|GetAs%20BP%20Player))
  (bind _defaultsceneroot (Variables|Default|GetDefaultSceneRoot))
  ;[1 1 1] Pick Up Event
  (Utilities|IsValid (Variables|/Game/Player/Blueprints/BP_Player.BP_Player_C|GetEquipedWeapon (Variables|Default|GetAs%20BP%20Player))
    (:Is%20Valid
      (Transformation|DetachFromActor (Variables|/Game/Player/Blueprints/BP_Player.BP_Player_C|GetEquipedWeapon (Variables|Default|GetAs%20BP%20Player)) "KeepRelative" "KeepRelative" "KeepRelative")
      (Transformation|SetActorLocationAndRotation (Variables|/Game/Player/Blueprints/BP_Player.BP_Player_C|GetEquipedWeapon (Variables|Default|GetAs%20BP%20Player)) (Transformation|GetWorldLocation _defaultsceneroot) (Transformation|GetWorldRotation _defaultsceneroot)))
    (:Is%20Not%20Valid
      _))
  (Variables|/Game/Player/Blueprints/BP_Player.BP_Player_C|SetEquipedWeapon _as_bp_player_2 self)
  (Transformation|AttachComponentToComponent (Variables|/Game/Player/Blueprints/BP_Player.BP_Player_C|GetFirstPersonMesh _as_bp_player_2) "SMG" "SnapToTarget" "SnapToTarget" "SnapToTarget" true)
  (Variables|/Game/Player/Blueprints/BP_Player.BP_Player_C|SetWeaponEquiped? (Variables|Default|GetAs%20BP%20Player) true)
  ;[1 0 0.8618] Bind Events
  ;;[1 1 1] Bind Use Item
  (EventDispatchers|BindEventtoOnUseItem _as_bp_player (EventDispatchers|CreateEvent :!event FireGun))
  ;;[1 1 1] Bind Reload
  (EventDispatchers|BindEventtoOnReload _as_bp_player (EventDispatchers|CreateEvent :!event Reload))
  ;;[1 1 1] Bind Stop Fire
  (EventDispatchers|BindEventtoStopFire _as_bp_player (delegate EventStopFiring))
  (Variables|/Game/Player/Blueprints/BP_Player.BP_Player_C|SetMP5%20Equiped? (Variables|Default|GetAs%20BP%20Player) true))

(event EventReload
  ;[1 1 1] Reload
  (if (and (!= (Variables|Default|GetAmmo) 0) (!= (Variables|Default|GetCurrent%20Mag) 30))
    (Utilities|FlowControl|DoOnce false :!label _label
      (:Completed
        (Variables|/Game/Player/Blueprints/BP_Player.BP_Player_C|SetReloading? (Variables|Default|GetAs%20BP%20Player) true)
        (Audio|PlaySound2D "/Game/Weapons/MP5/Sound/ReloadMP5.ReloadMP5" 1.0 1.0 0.0 0 0)
        (Animation|Montage|PlayMontage (Variables|/Game/Player/Blueprints/BP_Player.BP_Player_C|GetFirstPersonMesh (Variables|Default|GetAs%20BP%20Player)) "/Game/Player/Animations/Montages/FP_Reload_Montage.FP_Reload_Montage" 0.5
          (:then
            _)
          (:OnCompleted
            _))
        (Utilities|FlowControl|Delay 3.0)
        (CallFunction|ReloadSub)
        (Variables|/Game/Player/Blueprints/BP_Player.BP_Player_C|SetReloading? (Variables|Default|GetAs%20BP%20Player) false)
        (goto _label Reset)))))

(fn ConstructionScript
  (|CallParentFunction)
  (Variables|Default|SetCurrent%20Mag 30)
  (Variables|Default|SetAmmo 60)
  (Variables|Default|SetFire%20Rate 0.1))

(fn RandomRotCalc
  (params (InVec :type Vector))
  (bind _returnvalue (Math|Conversions|RotationFromXVector InVec))
  (bind _returnvalue_2 (Math|Random|RandomFloatinRange 0.0 3.6e+02))
  (bind (_x _y _z) (Math|Rotator|BreakRotIntoAxes _returnvalue))
  (return (Math|Rotator|MakeRotationfromAxes _x (Math|Vector|RotateVectorAroundAxis _y _returnvalue_2 _x) (Math|Vector|RotateVectorAroundAxis _z _returnvalue_2 _x))))

(fn UseAmmo
  (Variables|Default|SetCurrent%20Mag (Math|Integer|Clamp(Integer) (- (Variables|Default|GetCurrent%20Mag) 1) 0 30)))

(fn ReloadSub
  (LocalVariables|SetTemp%20Ammo (Variables|Default|GetAmmo))
  (Variables|Default|SetAmmo (Math|Integer|Clamp(Integer) (- (Variables|Default|GetAmmo) (- 30 (Variables|Default|GetCurrent%20Mag))) 0 (Variables|Default|GetAmmo)))
  (Variables|Default|SetCurrent%20Mag (+ (- (LocalVariables|GetTemp%20Ammo) (Variables|Default|GetAmmo)) (Variables|Default|GetCurrent%20Mag)))
  (if (Variables|Ammo|GetInfinite%20Ammo?)
    (Variables|Default|SetAmmo 999)))